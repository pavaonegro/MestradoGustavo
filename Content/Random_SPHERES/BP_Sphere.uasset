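; BP_Sphere is an interactable sphere actor with an active state and a sound that follows it.
; SetIsActive stores the flag and plays or stops the Audio component to match.
; OnInteract deactivates the sphere if it is active, then always calls OnSphereTriggered with itself, even when it was already inactive.
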(event `/Game/Random_SPHERES/BPI_Interaction.OnInteract`
  (`|ExecutionSequence`
    (:`then_0`
      (if (`self.IsActive`)
        (`self.SetIsActive` false)))
    (:`then_1`
      (`self.OnSphereTriggered` self))))

(fn `SetIsActive`
  (params (IsActive :type Boolean))
  (bind _audio (`self.Audio`))
  (bind _output_get (set `self.IsActive` IsActive))
  (if _output_get
    (`AudioComponent.Play` _audio 0.0)
    (else
      (`AudioComponent.Stop` _audio))))

(fn `UserConstructionScript`)